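; John is a playable character with walking, mouse-style look, jumping and a fuel-limited jetpack.
; Holding Jump on the ground jumps, then starts the jetpack after a delay, while pressing it airborne starts it immediately.
; Tick applies upward LaunchCharacter boosts and drains fuel time, which hitting JetpackFuel actors refills.
; The fall-compensated force is computed, but the launch uses a fixed value instead.
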(event EventTick
  (params (DeltaSeconds :type Float%20%28single-precision%29))
  (bind _jetpack_base_force (Variables|Default|GetJetpack%20Base%20Force))
  (if (and (Variables|Default|GetJetpack%20Active) (> (Variables|Default|GetJetpack%20Time) 0.0))
    (if (< (.z (Transformation|GetVelocity)) 0.0)
      (Variables|Default|SetJetpack%20Current%20Force (* _jetpack_base_force (Variables|Default|GetJetpack%20Negative%20Velocity%20Force%20Multiplier)))
      (else
        (Variables|Default|SetJetpack%20Current%20Force _jetpack_base_force)))
    (Character|LaunchCharacter (Math|Vector|MakeVector 0.0 0.0 (* DeltaSeconds 2e+03)) false false)
    (Variables|Default|SetJetpack%20Time (- (Variables|Default|GetJetpack%20Time) DeltaSeconds))))

(event Collision|EventHit
  (params (MyComp :type Primitive%20Component%20Object%20Reference) (Other :type Actor%20Object%20Reference) (OtherComp :type Primitive%20Component%20Object%20Reference) (bSelfMoved :type Boolean) (HitLocation :type Vector :default "0, 0, 0") (HitNormal :type Vector :default "0, 0, 0") (NormalImpulse :type Vector :default "0, 0, 0") (Hit :type Hit%20Result%20Structure%20%28by%20ref%29))
  ;[1 1 1] Pick up fuel
  (bind _asjetpack_fuel (Utilities|Casting|CastToJetpackFuel Other))
  (Variables|Default|SetJetpack%20Time (+ (Variables|Default|GetJetpack%20Time) (Variables|/Game/Blueprints/JetpackFuel.JetpackFuel_C|GetFuel%20Time _asjetpack_fuel)))
  (Actor|DestroyActor _asjetpack_fuel))

(event Input|ActionEvents|InputActionJump
  ;[1 1 1] Jump and activate jetpack
  (:Pressed
    (if (AI|Components|NavMovement|IsMovingonGround (Variables|Character|GetCharacterMovement))
      (Variables|Default|SetJump%20Active true)
      (Character|Jump)
      (Utilities|FlowControl|Delay (Variables|Default|GetJump%20To%20Jetpack%20Delay))
      (if (Variables|Default|GetJump%20Active)
        (Variables|Default|SetJetpack%20Active true))
      (else
        (Variables|Default|SetJetpack%20Active true))))
  (:Released
    (Variables|Default|SetJump%20Active false)
    (Variables|Default|SetJetpack%20Active false)))

(event Input|AxisEvents|InputAxisMoveRight
  (params (AxisValue :type Float%20%28single-precision%29))
  ;[1 1 1] Walk
  (Pawn|Input|AddMovementInput (Transformation|GetActorRightVector) AxisValue false))

(event Input|AxisEvents|InputAxisMoveForward
  (params (AxisValue :type Float%20%28single-precision%29))
  ;[1 1 1] Walk
  (Pawn|Input|AddMovementInput (Transformation|GetActorForwardVector) AxisValue false))

(event Input|AxisEvents|InputAxisLookUpDown
  (params (AxisValue :type Float%20%28single-precision%29))
  ;[1 1 1] Look around
  (Pawn|Input|AddControllerPitchInput AxisValue))

(event Input|AxisEvents|InputAxisLookRightLeft
  (params (AxisValue :type Float%20%28single-precision%29))
  ;[1 1 1] Look around
  (Pawn|Input|AddControllerYawInput AxisValue))

(fn ConstructionScript)